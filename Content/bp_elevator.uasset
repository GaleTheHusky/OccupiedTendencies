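; Elevator actor that moves its Cube platform between two points, A and B, when the player character type enters its trigger Box.
; A Character_Pawn overlap calls PlatformBegin, which restarts the Begin timeline and uses its track to lerp the Cube's relative location without sweeping.
; BeginPlay caches the player's Character_Pawn, though the movement logic never reads it.
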(event `self.ReceiveBeginPlay`
  (bind _ascharacter_pawn (cast `/Game/Interaction/Blueprints/Pawn/Player/Character_Pawn` (`GameplayStatics.GetPlayerCharacter` 0)))
  (set `self.As Character Pawn` _ascharacter_pawn))

(event `Platform Begin`
  (bind (_direction _newtrack_0) (`Timeline|begin` :!via `PlayFromStart`)
    (:`Update`
      (`SceneComponent.K2_SetRelativeLocation` (`self.Cube`) (`KismetMathLibrary.VLerp` (`self.A`) (`self.B`) _newtrack_0) false false))))

(event `self.Box.OnComponentBeginOverlap`
  (params (OverlappedComponent :type "PrimitiveComponent Object Reference") (OtherActor :type "Actor Object Reference") (OtherComp :type "PrimitiveComponent Object Reference") (OtherBodyIndex :type Integer) (bFromSweep :type Boolean) (SweepResult :type "HitResult Structure (by ref)"))
  (cast `/Game/Interaction/Blueprints/Pawn/Player/Character_Pawn` OtherActor)
  (`self.Platform Begin`))

(fn `UserConstructionScript`)